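; Sliding door Blueprint that opens and closes in response to an optional linked button and lock, or through its Open and Close events.
; Timed component moves slide the door between two positions, each direction cancelling the other, guarded by open and locked flags.
; Button and lock events also update optional status lights, and unlocking opens the door directly when no button is linked.
; Construction copies the door material and starts it locked if a lock is assigned.
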(event `OnDoorOpened`
  ;[1 1 1] Door Opened
  (`KismetSystemLibrary.PrintText` "Door Open" false true (struct :`G` 0.66 :`B` 1.0 :`A` 1.0) 10.0)
  (if (and (not (`self.IsOpened`)) (not (`self.IsLocked`)))
    (`self.OnCancelDoorClosed`)
    (set `self.IsOpened` true)
    (`KismetSystemLibrary.MoveComponentTo` (`self.Door`) (`self.OpenPosition`) (struct) false false (`self.AnimationDuration`) :!label _label)))

(event `OnCancelDoorOpened`
  ;[1 1 1] Door Opened
  (goto _label :!via `Stop`))

(event `OnDoorClosed`
  ;[1 1 1] Door closed
  (`KismetSystemLibrary.PrintText` "Door Close" false true (struct :`G` 0.66 :`B` 1.0 :`A` 1.0) 10.0)
  (if (and (`self.IsOpened`) (not (`self.IsLocked`)))
    (set `self.IsOpened` false)
    (`self.OnCancelDoorOpened`)
    (`KismetSystemLibrary.MoveComponentTo` (`self.Door`) (`self.ClosePosition`) (struct) false false (`self.AnimationDuration`) :!label _label_2)))

(event `OnCancelDoorClosed`
  ;[1 1 1] Door closed
  (goto _label_2 :!via `Stop`))

(event `self.Button.ButtonPressed`
  ;[1 1 1] Events associated with the button
  (`self.OnDoorOpened`)
  (if (!= (`self.ButtonLightStatus`) null)
    (`/Game/Environment/LightStatus_BP.OnAllowed` (`self.ButtonLightStatus`))))

(event `self.Button.ButtonReleased`
  ;[1 1 1] Events associated with the button
  (`self.OnDoorClosed`)
  (if (!= (`self.ButtonLightStatus`) null)
    (`/Game/Environment/LightStatus_BP.OnDenied` (`self.ButtonLightStatus`))))

(event `self.Lock.Unlocked`
  ;[1 1 1] Event associated with the lock
  (set `self.IsLocked` false)
  (if (!= (`self.LockLightStatus`) null)
    (`/Game/Environment/LightStatus_BP.OnAllowed` (`self.LockLightStatus`)))
  (if (== (`self.Button`) null)
    (`self.OnDoorOpened`)))

(event `Open`
  ;[1 1 1] Actions
  (`self.OnDoorOpened`))

(event `Close`
  ;[1 1 1] Actions
  (`self.OnDoorClosed`))

(fn `UserConstructionScript`
  (`PrimitiveComponent.SetMaterial` (`self.Door`) 0 (`PrimitiveComponent.GetMaterial` (`self.StaticMeshComponent`) 0))
  (if (!= (`self.Lock`) null)
    (set `self.IsLocked` true)))