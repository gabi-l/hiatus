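; Time plate actor that triggers a timed rewind on a Runner stepping onto it.
; On authority, trigger overlap passes the plate's time and rewind durations and itself to the Runner, marks it occupied and active, and applies the ghost material.
; RewindFinished clears the active state and shows a red unusable material.
; A Runner leaving the inactive, occupied plate frees it and restores its normal material.
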(event `MaterialChanged`
  (params (Material :type "Material Object Reference"))
  ;[1 1 1] Occurs when the material changed
  (`PrimitiveComponent.SetMaterial` (`self.Plate`) 0 Material))

(event `self.TriggerBoxEnter.OnComponentBeginOverlap`
  (params (OverlappedComponent :type "PrimitiveComponent Object Reference") (OtherActor :type "Actor Object Reference") (OtherComp :type "PrimitiveComponent Object Reference") (OtherBodyIndex :type Integer) (bFromSweep :type Boolean) (SweepResult :type "HitResult Structure (by ref)"))
  (`/Engine/EditorBlueprintResources/ActorMacros.Switch Has Authority`
    (:`Authority`
      (if (and (not (`self.IsOccupied`)) (not (`self.IsActive`)))
        ;[1 1 1] Activate the plate and trigger runner
        (bind _asrunner (cast `/Game/Characters/Runner` OtherActor))
        (`/Game/Characters/Runner.PlateActivated` _asrunner (`self.Time`) (`self.RewindDuration`) self)
        (set `self.IsOccupied` true)
        (`self.MaterialChanged` "/Game/Assets/Materials/Ghost.Ghost")
        (set `self.IsActive` true)))))

(event `self.TriggerBoxLeave.OnComponentEndOverlap`
  (params (OverlappedComponent :type "PrimitiveComponent Object Reference") (OtherActor :type "Actor Object Reference") (OtherComp :type "PrimitiveComponent Object Reference") (OtherBodyIndex :type Integer))
  (`/Engine/EditorBlueprintResources/ActorMacros.Switch Has Authority`
    (:`Authority`
      (cast `/Game/Characters/Runner` OtherActor)
      (if (and (not (`self.IsActive`)) (`self.IsOccupied`))
        ;[1 1 1] Make plate available again
        (set `self.IsOccupied` false)
        (`self.MaterialChanged` "/Game/Assets/Materials/TimePlate_Mat.TimePlate_Mat")))))

(event `RewindFinished`
  ;[1 1 1] Deactivate plate and set material to unusable
  (set `self.IsActive` false)
  (`self.MaterialChanged` "/Game/Assets/Materials/RedLightMaterial.RedLightMaterial"))

(fn `UserConstructionScript`)