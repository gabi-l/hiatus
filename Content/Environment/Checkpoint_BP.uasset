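; Checkpoint actor that a Runner activates by overlapping its zone, with the server reporting its ID to the Runner.
; Activation plays a sound, swaps the light material to a dynamic instance and sets the particle spawn rate to zero.
; While active, Tick pulses the light parameter along a sharpened sine wave between min and max.
; A multicast Deactivate restores the idle material and particles.
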(event `self.CheckpointZone.OnComponentBeginOverlap`
  (params (OverlappedComponent :type "PrimitiveComponent Object Reference") (OtherActor :type "Actor Object Reference") (OtherComp :type "PrimitiveComponent Object Reference") (OtherBodyIndex :type Integer) (bFromSweep :type Boolean) (SweepResult :type "HitResult Structure (by ref)"))
  ;[1 1 1] Runner touches checkpoint
  (bind _asrunner (cast `/Game/Characters/Runner` OtherActor))
  (if (not (`self.Activated`))
    (set `self.Activated` true)
    (`AudioComponent.Play` (`self.TriggerSound`) 0.0)
    (`PrimitiveComponent.SetMaterial` (`self.StaticMesh`) 1 (`self.Lights`))
    (`self.Particles Activation`)
    (`/Engine/EditorBlueprintResources/ActorMacros.Switch Has Authority`
      (:`Authority`
        (`/Game/Characters/Runner.ReachedCheckpoint` _asrunner (`self.ID`))))))

(event `self.ReceiveTick`
  (params (DeltaSeconds :type "Float (single-precision)"))
  ;[1 1 1] Oscillate
  (if (`self.Activated`)
    (bind _output_get (set `self.Oscillation` (+ (* DeltaSeconds (`self.Frequency`) (`KismetMathLibrary.GetPI`) 2.0) (`self.Oscillation`))))
    (`MaterialInstanceDynamic.SetScalarParameterValue` (`self.Lights`) "Light" (`KismetMathLibrary.Lerp` (`self.MinLight`) (`self.MaxLight`) (`KismetMathLibrary.MultiplyMultiply_FloatFloat` (/ (+ (`KismetMathLibrary.Sin` _output_get) 1.0) 2.0) 3.0)))))

(event `Deactivate`
  ;[1 1 1] Deactivate
  (`self.Deactivate Multicast`))

(event `Deactivate Multicast`
  ;[1 1 1] Deactivate
  (set `self.Activated` false)
  (`PrimitiveComponent.SetMaterial` (`self.StaticMesh`) 1 "/Game/Assets/Materials/MT_CheckpointLight.MT_CheckpointLight")
  (set `self.Oscillation` 0.0)
  (`ParticleSystemComponent.SetFloatParameter` (`self.ParticleSystem`) "SpawnRate" 30.0))

(event `Particles Activation`
  ;[1 1 1] Comment
  (`ParticleSystemComponent.SetFloatParameter` (`self.ParticleSystem`) "SpawnRate" 0.0))

(fn `UserConstructionScript`
  (bind _returnvalue (`KismetMaterialLibrary.CreateDynamicMaterialInstance` "/Game/Assets/Materials/MT_Checkpoint_LightPassed.MT_Checkpoint_LightPassed"))
  (set `self.Lights` _returnvalue)
  (`ParticleSystemComponent.SetFloatParameter` (`self.ParticleSystem`) "SpawnRate" 30.0))