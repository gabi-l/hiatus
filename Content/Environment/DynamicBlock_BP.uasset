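; DynamicBlock_BP is an environment block that moves between two placed transforms in response to its Activator's Activate and Deactivate events.
; BeginPlay stores the Start and Destination transforms, then destroys the Destination component, which serves only as a target marker.
; Activator events set a Pressed flag that drives a clamped Alpha on Tick, with separate forward and backward durations.
; Start's world transform is lerped by Alpha, so movement can reverse mid-travel.
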(event `self.ReceiveBeginPlay`
  ;[1 1 1] Startup
  (`|ExecutionSequence`
    (:`then_0`
      ;;[1 1 1] Save transforms
      (set `self.StartTransform` (`SceneComponent.K2_GetComponentToWorld` (`self.Start`)))
      (set `self.DestinationTransform` (`SceneComponent.K2_GetComponentToWorld` (`self.Destination`))))
    (:`then_1`
      ;;[1 1 1] Remove destination
      (`ActorComponent.K2_DestroyComponent` (`self.Destination`)))))

(event `self.Activator.Activate`
  ;[1 1 1] Receive input
  (`self.ChangeState` true))

(event `ChangeState`
  (params (IsPressed :type Boolean))
  (set `self.Pressed` IsPressed))

(event `self.Activator.Deactivate`
  ;[1 1 1] Receive input
  (`self.ChangeState` false))

(event `self.ReceiveTick`
  (params (DeltaSeconds :type "Float (single-precision)"))
  ;[1 1 1] Interpolate
  (`self.LerpBlock` DeltaSeconds))

(event `LerpBlock`
  (params (DeltaSecond :type "Float (double-precision)"))
  (set `self.Alpha` (`KismetMathLibrary.FClamp` (+ (* DeltaSecond (`KismetMathLibrary.SelectFloat` (/ 1.0 (`self.Forward Time (sec)`)) (/ -1.0 (`self.Backward Time (sec)`)) (`self.Pressed`))) (`self.Alpha`))))
  (`SceneComponent.K2_SetWorldTransform` (`self.Start`) (`KismetMathLibrary.TLerp` (`self.StartTransform`) (`self.DestinationTransform`) (`self.Alpha`)) false false))

(fn `UserConstructionScript`)