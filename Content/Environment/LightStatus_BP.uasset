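; Status light Blueprint that shows an allowed or denied state by swapping the material on its Light component.
; OnAllowed and OnDenied events each set the allow or deny status material on the first material slot.
; The construction script calls one of these events based on the IsAllowed flag to set the initial look.
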(event `OnAllowed`
  ;[1 1 1] Allow status
  (`PrimitiveComponent.SetMaterial` (`self.Light`) 0 (`self.AllowStatusMaterial`)))

(event `OnDenied`
  ;[1 1 1] Deny status
  (`PrimitiveComponent.SetMaterial` (`self.Light`) 0 (`self.DenyStatusMaterial`)))

(fn `UserConstructionScript`
  (if (`self.IsAllowed`)
    (`self.OnAllowed`)
    (else
      (`self.OnDenied`))))