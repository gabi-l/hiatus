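; A sizable wall actor that can be hidden through SetTranslucentObjectVisibility, either by fading or by an instant toggle.
; The construction script gives opaque and translucent twin components the same mesh and scale, with dynamic material instances on the translucent one.
; Tick moves FadeState over FadeTime to drive Opacity, showing the opaque twin only at full opacity.
; Tick also clears Hidden after applying it, so hiding relies on repeated requests.
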(event `Set Translucent Object Visibility`
  (params (Hidden :type Boolean) (Fade :type Boolean))
  ;[1 1 1] Set Visibility
  (set `self.StateChanged` (!= Hidden (`self.Hidden`)))
  (set `self.Hidden` Hidden)
  (set `self.ShouldFade` Fade))

(event `self.ReceiveTick`
  (params (DeltaSeconds :type "Float (single-precision)"))
  (bind _returnvalue (`KismetMathLibrary.NearlyEqual_FloatFloat` (`self.Fade State`) 1.0 0.001))
  ;[1 1 1] Event Tick
  (if (`self.ShouldFade`)
    (`self.Set Fade State` DeltaSeconds)
    (if (!= _returnvalue (`self.IsOpaque`))
      (bind _output_get (set `self.IsOpaque` _returnvalue))
      (`self.Set SwappedWall Visibility State` _output_get)
      (set `self.Hidden` false)
      (elif (not _returnvalue)
        (`self.Set Opacity Parameters`)
        (set `self.Hidden` false)))
    (elif (`self.StateChanged`)
      (`self.Set Hard Wall Visibility State` (not (`self.Hidden`)))
      (set `self.Hidden` false))))

(event `Set Fade State`
  (params (`Delta Seconds` :type "Float (double-precision)"))
  ;[1 1 1] Set Fade State
  (set `self.Fade State` (`KismetMathLibrary.Lerp` (`KismetMathLibrary.SelectFloat` (`self.Min Translucency`) 0.0 (`self.ShouldFade`)) (`KismetMathLibrary.SelectFloat` (`self.Max Translucency`) 1.0 (`self.ShouldFade`)) (`KismetMathLibrary.FClamp` (+ (* (/ `Delta Seconds` (`self.Fade Time`)) (`KismetMathLibrary.SelectFloat` -1.0 1.0 (`self.Hidden`))) (`self.Fade State`))))))

(event `Set SwappedWall Visibility State`
  (params (Opaque :type Boolean))
  ;[1 1 1] Set Swapped Wall Visibility State
  (`SceneComponent.SetVisibility` (`self.OpaqueMesh`) Opaque false)
  (`SceneComponent.SetVisibility` (`self.TranslucentMesh`) (not Opaque) false))

(event `Set Hard Wall Visibility State`
  (params (Opaque :type Boolean))
  ;[1 1 1] Set Hard Wall Visibility State
  (`SceneComponent.SetVisibility` (`self.OpaqueMesh`) Opaque false)
  (`SceneComponent.SetVisibility` (`self.TranslucentMesh`) false false))

(event `Set Opacity Parameters`
  ;[1 1 1] Set Opacity Parameters
  (for _array_element (`self.DynamicMaterials`)
    (`MaterialInstanceDynamic.SetScalarParameterValue` _array_element "Opacity" (`self.Fade State`))))

(fn `UserConstructionScript`
  (bind _returnvalue (/ (`self.Size`) (`KismetMathLibrary.MakeVector` 100.0 100.0 100.0)))
  (`|ExecutionSequence`
    (:`then_0`
      ;[1 1 1] Set Static Meshes
      (`StaticMeshComponent.SetStaticMesh` (`self.OpaqueMesh`) (`self.Mesh`))
      (`StaticMeshComponent.SetStaticMesh` (`self.TranslucentMesh`) (`self.Mesh`)))
    (:`then_1`
      ;[1 1 1] Set Meshes Visibility
      (`SceneComponent.SetVisibility` (`self.OpaqueMesh`) true false)
      (`SceneComponent.SetVisibility` (`self.TranslucentMesh`) false false))
    (:`then_2`
      ;[1 1 1] Set Meshes Scales
      (`SceneComponent.SetRelativeScale3D` (`self.OpaqueMesh`) _returnvalue)
      (`SceneComponent.SetRelativeScale3D` (`self.TranslucentMesh`) _returnvalue))
    (:`then_3`
      ;[1 1 1] Set Opaque Material
      (for (_array_element _array_index) (`self.OpaqueMaterialInstances`)
        (`PrimitiveComponent.SetMaterial` (`self.OpaqueMesh`) _array_index _array_element)))
    (:`then_4`
      ;[1 1 1] Set Dynamic Material
      (for (_array_element_2 _array_index_2) (`self.TranslucentMaterialInstances`)
        (bind _returnvalue_2 (`PrimitiveComponent.CreateDynamicMaterialInstance` (`self.TranslucentMesh`) _array_index_2 _array_element_2))
        (`KismetArrayLibrary.Array_Add` (`self.DynamicMaterials`) _returnvalue_2)))))