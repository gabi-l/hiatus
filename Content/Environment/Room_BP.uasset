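; Room Blueprint with a numbered, lockable door that slides open once when its collision box is overlapped while unlocked.
; The construction script writes the room number to both text components and applies the initial lock state.
; A child Lock_BP's Unlocked event clears the lock at runtime.
; SetLockStatus turns the child Light_BP red or green and toggles the lock indicator's visibility.
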(event `self.ReceiveBeginPlay`
  ;[1 1 1] Binds the unlocked event
  (bind _aslock_bp (cast `/Game/Environment/Lock_BP` (`ChildActorComponent.ChildActor` (`self.LockIndicator`))))
  (add `/Game/Environment/Lock_BP.Unlocked` _aslock_bp (delegate `DoorUnlocked`)))

(event `DoorUnlocked`
  ;[1 1 1] Unlocks the door
  (`self.SetLockStatus` false))

(event `self.CollisionBox.OnComponentBeginOverlap`
  (params (OverlappedComponent :type "PrimitiveComponent Object Reference") (OtherActor :type "Actor Object Reference") (OtherComp :type "PrimitiveComponent Object Reference") (OtherBodyIndex :type Integer) (bFromSweep :type Boolean) (SweepResult :type "HitResult Structure (by ref)"))
  (bind _door (`self.Door`))
  ;[1 1 1] Opens the door
  (if (and (not (`self.IsLocked`)) (not (`self.IsDoorOpened`)))
    (`SceneComponent.SetVisibility` (`self.LockIndicator`) false false)
    (set `self.IsDoorOpened` true)
    (`KismetSystemLibrary.MoveComponentTo` _door (+ (`SceneComponent.RelativeLocation` _door) (180.0 0.0 0.0)) (struct) false false 2.0)))

(fn `SetLockStatus`
  (params (IsLocked :type Boolean))
  (set `self.IsLocked` IsLocked)
  (bind _aslight_bp (cast `/Game/Environment/Light_BP` (`ChildActorComponent.ChildActor` (`self.LightIndicator`))))
  ;[1 1 1] Sets the light color
  (if (`self.IsLocked`)
    (set `self.LightColor` (struct :`R` 1.0 :`A` 1.0))
    (else
      (set `self.LightColor` (struct :`G` 1.0 :`A` 1.0))))
  (`LightComponent.SetLightColor` (`/Game/Environment/Light_BP.LightIndicator` _aslight_bp) (`self.LightColor`) true)
  ;[1 1 1] Hides or shows the lock indicator
  (`SceneComponent.SetVisibility` (`self.LockIndicator`) (`self.IsLocked`) false))

(fn `UserConstructionScript`
  (bind _returnvalue (`KismetTextLibrary.Conv_StringToText` (`self.RoomNumber`)))
  ;[1 1 1] Sets the room number
  (`TextRenderComponent.K2_SetText` (`self.RoomNumberText`) _returnvalue)
  (`TextRenderComponent.K2_SetText` (`self.FloorNumber`) _returnvalue)
  (`self.SetLockStatus` (`self.IsLocked`)))