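; Lock actor that hides its sphere, disables its collision and fires Unlocked when the replicated IsLocked flag clears.
; Pressing it completes the selection action immediately if no password is set, otherwise it enables input and shows a PasswordInput_BP widget.
; Gamepad face buttons become A/B/X/Y characters, and a submission matching the password completes the action.
; CompleteAction clears IsLocked, letting the RepNotify handle the visible unlock.
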(event `self.ReceiveBeginPlay`
  ;[1 1 1] Adds the password input in the viewport
  (bind _returnvalue (`|CreateWidget` "/Game/UI/Game/PasswordInput_BP.PasswordInput_BP_C"))
  (bind _output_get (set `self.PasswordInput` _returnvalue))
  (`Widget.SetVisibility` _output_get "Collapsed")
  (`UserWidget.AddToViewport` (`self.PasswordInput`) 100)
  (set `/Game/UI/Game/PasswordInput_BP.ExpectedPassword` (`self.Password`) (`self.PasswordInput`))
  (add `/Game/UI/Game/PasswordInput_BP.PasswordSubmitted` (`self.PasswordInput`) (delegate `PasswordSubmitted`)))

(event `InputAction|Password`
  (params (Key :type "Key Structure" :default "AnyKey"))
  ;[1 1 1] Gets the input from the controller
  (:`Pressed`
    (bind _char (`self.GetCharFromKey` Key))
    (`/Game/UI/Game/PasswordInput_BP.AddPasswordChar` (`self.PasswordInput`) _char)))

(event `PasswordSubmitted`
  (params (PasswordSpecified :type String))
  ;[1 1 1] Checks if the password is correct
  (`self.DisableInput` (`GameplayStatics.GetPlayerController` 0))
  (`KismetSystemLibrary.Delay` 0.4)
  (`Widget.SetVisibility` (`self.PasswordInput`) "Hidden")
  (if (`KismetStringLibrary.EqualEqual_StrStr` PasswordSpecified (`self.Password`))
    (`self.SelectionActionCompleted`)))

(fn `CompleteAction`
  (params (Param :type Boolean))
  (returns (Return :type Boolean))
  (set `self.IsLocked` false)
  (return false))

(fn `GetCharFromKey`
  (params (Key :type "Key Structure" :default "AnyKey"))
  (returns (Char :type String))
  (if (== Key "Gamepad_FaceButton_Bottom")
    (return "A")
    (elif (== Key "Gamepad_FaceButton_Right")
      (return "B")
      (elif (== Key "Gamepad_FaceButton_Left")
        (return "X")
        (else
          (return "Y"))))))

(fn `GetInformation`
  (params (Param :type Boolean))
  (returns (Infos :type String))
  (return (`self.InformationText`)))

(fn `OnRep_IsLocked`
  (if (not (`self.IsLocked`))
    (`SceneComponent.SetVisibility` (`self.Sphere`) false true)
    (`PrimitiveComponent.SetCollisionResponseToAllChannels` (`self.Sphere`) "ECR_Ignore")
    (`self.Unlocked`)))

(fn `PressAction`
  (params (Param :type Boolean))
  (returns (Return :type Boolean))
  (if (`KismetStringLibrary.NotEqual_StrStr` (`self.Password`))
    (`self.EnableInput` (`GameplayStatics.GetPlayerController` 0))
    (`/Game/UI/Game/PasswordInput_BP.Reset` (`self.PasswordInput`))
    (`Widget.SetVisibility` (`self.PasswordInput`) "Visible")
    (return false)
    (else
      (`self.SelectionActionCompleted`)
      (return false))))

(fn `UserConstructionScript`)