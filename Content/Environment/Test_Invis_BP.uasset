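; Test blueprint that previews a blend between two materials on its Cube component, apparently for an invisibility effect.
; The construction script creates a dynamic material instance from Material1, interpolates its parameters between Material1 and Material2 by Alpha, and applies it to the first material slot.
; The blend updates only when construction runs, as the event graph holds just disabled default events.
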(fn `UserConstructionScript`
  (bind _returnvalue (`PrimitiveComponent.CreateDynamicMaterialInstance` (`self.Cube`) 0 (`self.Material 1`)))
  (set `self.DynamicMaterial` _returnvalue)
  (`MaterialInstanceDynamic.K2_InterpolateMaterialInstanceParams` (`self.DynamicMaterial`) (`self.Material 1`) (`self.Material 2`) (`self.Alpha`))
  (`PrimitiveComponent.SetMaterial` (`self.Cube`) 0 (`self.DynamicMaterial`)))