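; Arrow_BP is an indicator arrow that loops an eased bob between two positions while enabled, with ConditionalDisplay receiving its Character setting at construction.
; A trigger box overlap, an Activator activation or a button press disables it, on the authority only.
; The IsEnabled RepNotify then hides the scene component and its children, and the animation loop stops at its next check.
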(event `self.ReceiveBeginPlay`
  ;[1 1 1] Animation
  (if (`self.IsEnabled`) :!label _label
    (`KismetSystemLibrary.MoveComponentTo` (`self.Arrow`) (`self.TopPosition`) (struct) true true (`self.AnimationDuration`))
    (if (`self.IsEnabled`)
      (`KismetSystemLibrary.MoveComponentTo` (`self.Arrow`) (`self.EndPosition`) (struct) true true (`self.AnimationDuration`))
      (goto _label))))

(event `self.TriggerBox.OnActorBeginOverlap`
  (params (OverlappedActor :type "Actor Object Reference") (OtherActor :type "Actor Object Reference"))
  ;[1 1 1] Hides arrow
  (`/Engine/EditorBlueprintResources/ActorMacros.Switch Has Authority`
    (:`Authority`
      (set `self.IsEnabled` false))))

(event `self.Activator.Activate`
  ;[1 1 1] Hides arrow
  (`/Engine/EditorBlueprintResources/ActorMacros.Switch Has Authority`
    (:`Authority`
      (set `self.IsEnabled` false))))

(event `self.Button.ButtonPressed`
  ;[1 1 1] Hides arrow
  (`/Engine/EditorBlueprintResources/ActorMacros.Switch Has Authority`
    (:`Authority`
      (set `self.IsEnabled` false))))

(fn `OnRep_IsEnabled`
  (`SceneComponent.SetVisibility` (`self.Scene`) false true))

(fn `UserConstructionScript`
  (set `/Game/Shared/ConditionalDisplay.Character` (`self.Character`) (`self.ConditionalDisplay`)))