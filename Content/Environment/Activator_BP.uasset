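; Interactable activator actor with a gear billboard that broadcasts activate and deactivate events when used.
; An optional linked Button gates it: the server disables it at start, and it is enabled only while the button is pressed.
; The disabled flag's RepNotify swaps the gear material and toggles whether the sphere blocks a custom trace channel.
; CompleteAction shows the animated gear and activates if enabled, while ReleaseAction restores the material and deactivates.
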(event `self.ReceiveBeginPlay`
  ;[1 1 1] Initialization
  (`/Engine/EditorBlueprintResources/ActorMacros.Switch Has Authority`
    (:`Authority`
      (if (!= (`self.Button`) null)
        (set `self.IsDisabled` true)))))

(event `self.Button.ButtonPressed`
  ;[1 1 1] Button logic
  (set `self.IsDisabled` false))

(event `self.Button.ButtonReleased`
  ;[1 1 1] Button logic
  (set `self.IsDisabled` true))

(event `UpdateMaterial`
  (params (Material :type "Material Object Reference"))
  ;[1 1 1] Update material
  (`PrimitiveComponent.SetMaterial` (`self.Billboard`) 0 Material))

(fn `CompleteAction`
  (params (Param :type Boolean))
  (returns (Return :type Boolean))
  (if (not (`self.IsDisabled`))
    (`self.UpdateMaterial` "/Game/Assets/Materials/AnimatedGearMaterial.AnimatedGearMaterial")
    (`self.Activate`)
    (return false)))

(fn `GetInformation`
  (params (Param :type Boolean))
  (returns (Infos :type String))
  (return (`self.InformationText`)))

(fn `OnRep_IsLocked`
  (if (`self.IsDisabled`)
    (`PrimitiveComponent.SetMaterial` (`self.Billboard`) 0 "/Game/Assets/Materials/GearDisabledMaterial.GearDisabledMaterial")
    (`PrimitiveComponent.SetCollisionResponseToChannel` (`self.Sphere`) "ECC_GameTraceChannel1" "ECR_Ignore")
    (else
      (`PrimitiveComponent.SetMaterial` (`self.Billboard`) 0 "/Game/Assets/Materials/GearMaterial.GearMaterial")
      (`PrimitiveComponent.SetCollisionResponseToChannel` (`self.Sphere`) "ECC_GameTraceChannel1" "ECR_Block"))))

(fn `PressAction`
  (params (Param :type Boolean))
  (returns (Return :type Boolean))
  (return false))

(fn `ReleaseAction`
  (params (Param :type Boolean))
  (returns (Return :type Boolean))
  (if (`self.IsDisabled`)
    (`self.UpdateMaterial` "/Game/Assets/Materials/GearDisabledMaterial.GearDisabledMaterial")
    (else
      (`self.UpdateMaterial` "/Game/Assets/Materials/GearMaterial.GearMaterial")))
  (`self.Deactivate`)
  (return false))

(fn `UserConstructionScript`)