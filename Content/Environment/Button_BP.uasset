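; Pressure button Blueprint that presses when an actor other than a Ghost enters its trigger and releases when no Runner or Clone remains.
; Overlaps are handled only with authority.
; MoveComponentTo animates the button between press and release positions, each direction cancelling the other, swapping materials and calling pressed/released events when moves complete.
; The construction script positions the button from its initial IsPressed state.
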(event `OnButtonPressed`
  ;[1 1 1] Button pressed
  (if (not (`self.IsPressed`))
    (`self.OnCancelButtonReleased`)
    (set `self.IsPressed` true)
    (`KismetSystemLibrary.MoveComponentTo` (`self.Button`) (`self.PressPosition`) (struct) false false (`self.AnimationDuration`) :!label _label)
    (if (`self.IsPressed`)
      (`PrimitiveComponent.SetMaterial` (`self.Button`) 0 (`self.ButtonPressedMaterial`))
      (`self.ButtonPressed`))))

(event `OnCancelButtonPressed`
  ;[1 1 1] Button pressed
  (goto _label :!via `Stop`))

(event `OnButtonReleased`
  ;[1 1 1] Button released
  (if (`self.IsPressed`)
    (set `self.IsPressed` false)
    (`self.OnCancelButtonPressed`)
    (`PrimitiveComponent.SetMaterial` (`self.Button`) 0 (`self.ButtonReleasedMaterial`))
    (`KismetSystemLibrary.MoveComponentTo` (`self.Button`) (`self.ReleasePosition`) (struct) false false (`self.AnimationDuration`) :!label _label_2)
    (if (not (`self.IsPressed`))
      (`self.ButtonReleased`))))

(event `OnCancelButtonReleased`
  ;[1 1 1] Button released
  (goto _label_2 :!via `Stop`))

(event `self.Trigger.OnComponentBeginOverlap`
  (params (OverlappedComponent :type "PrimitiveComponent Object Reference") (OtherActor :type "Actor Object Reference") (OtherComp :type "PrimitiveComponent Object Reference") (OtherBodyIndex :type Integer) (bFromSweep :type Boolean) (SweepResult :type "HitResult Structure (by ref)"))
  ;[1 1 1] Trigger box events
  (`/Engine/EditorBlueprintResources/ActorMacros.Switch Has Authority`
    (:`Authority`
      (cast `/Game/Characters/Ghost_BP` OtherActor ; Desole pour le bug fix laid
        (:`CastFailed`
          (`self.OnButtonPressed`))))))

(event `self.Trigger.OnComponentEndOverlap`
  (params (OverlappedComponent :type "PrimitiveComponent Object Reference") (OtherActor :type "Actor Object Reference") (OtherComp :type "PrimitiveComponent Object Reference") (OtherBodyIndex :type Integer))
  ;[1 1 1] Trigger box events
  (`/Engine/EditorBlueprintResources/ActorMacros.Switch Has Authority`
    (:`Authority`
      (cast `/Game/Characters/Ghost_BP` OtherActor
        (:`CastFailed`
          (bind _actors (`self.KeepRunnerAndClone` (`PrimitiveComponent.GetOverlappingActors` (`self.Trigger`) null)))
          (if (not (> (`KismetArrayLibrary.Array_Length` _actors) 0))
            (`self.OnButtonReleased`)))))))

(fn `KeepRunnerAndClone`
  (params (Actor :type "Array of Actor Object Reference"))
  (returns (Actors :type "Array of Actor Object Reference"))
  (locals (ActorsToRemove :type "Array of Actor Object Reference"))
  ;[1 1 1] Get all actors to remove from the list
  (for _array_element Actor
    (bind _returnvalue (`GameplayStatics.GetObjectClass` _array_element))
    (if (!= _returnvalue "/Game/Characters/Clone_BP.Clone_BP_C")
      (if (!= _returnvalue "/Game/Characters/Runner.Runner_C")
        (`KismetArrayLibrary.Array_Add` (`local.ActorsToRemove`) _array_element))))
  ;[1 1 1] Remove actor from the list
  (for _array_element_2 (`local.ActorsToRemove`)
    (`KismetArrayLibrary.Array_RemoveItem` Actor _array_element_2))
  (return Actor))

(fn `UserConstructionScript`
  (if (`self.IsPressed`)
    (`PrimitiveComponent.SetMaterial` (`self.Button`) 0 null)
    (`SceneComponent.K2_SetRelativeLocation` (`self.Button`) (`self.PressPosition`) false false)
    (else
      (`PrimitiveComponent.SetMaterial` (`self.Button`) 0 null)
      (`SceneComponent.K2_SetRelativeLocation` (`self.Button`) (`self.ReleasePosition`) false false))))