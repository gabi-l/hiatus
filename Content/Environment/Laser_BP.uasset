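; Laser hazard that kills any Runner overlapping its box while enabled.
; The server handles the overlap kill and toggles IsEnabled from an Activator, where activation turns the laser off and deactivation turns it back on.
; An OnRep on IsEnabled shows or hides the beam particles.
; The construction script sizes the particle beam length from the box's scaled X extent while keeping particle world scale at one.
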(event `self.Box.OnComponentBeginOverlap`
  (params (OverlappedComponent :type "PrimitiveComponent Object Reference") (OtherActor :type "Actor Object Reference") (OtherComp :type "PrimitiveComponent Object Reference") (OtherBodyIndex :type Integer) (bFromSweep :type Boolean) (SweepResult :type "HitResult Structure (by ref)"))
  ;[1 1 1] Runner touches laser
  (`/Engine/EditorBlueprintResources/ActorMacros.Switch Has Authority`
    (:`Authority`
      (if (`self.IsEnabled`)
        (bind _asrunner (cast `/Game/Characters/Runner` OtherActor))
        (`/Game/Characters/Runner.Die` _asrunner)))))

(event `self.Activator.Activate`
  ;[1 1 1] Activator logic
  (`/Engine/EditorBlueprintResources/ActorMacros.Switch Has Authority`
    (:`Authority`
      (set `self.IsEnabled` false))))

(event `self.Activator.Deactivate`
  ;[1 1 1] Activator logic
  (`/Engine/EditorBlueprintResources/ActorMacros.Switch Has Authority`
    (:`Authority`
      (set `self.IsEnabled` true))))

(fn `OnRep_IsEnabled`
  (`SceneComponent.SetVisibility` (`self.LaserParticles`) (`self.IsEnabled`) true))

(fn `UserConstructionScript`
  (bind _box (`self.Box`))
  ;[1 1 1] Adjust laser scale
  (`ParticleSystemComponent.SetFloatParameter` (`self.LaserParticles`) "LaserLength" (* (.x (`BoxComponent.BoxExtent` _box)) (.x (`SceneComponent.K2_GetComponentScale` _box)) 2.0))
  (`SceneComponent.SetWorldScale3D` (`self.LaserParticles`) (1.0 1.0 1.0)))