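; Laser field Blueprint that builds a vertical stack of Laser_BP actors within a box volume.
; Its construction script adds LaserCount child actor components, interpolating their height evenly from the bottom to the top of the box's extent.
; Each laser's relative Z scale is the inverse of the box's world Z scale, countering vertical stretching when the field is scaled.
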(fn `UserConstructionScript`
  (bind _box (`self.Box`))
  (bind _returnvalue (- (`self.LaserCount`) 1))
  (bind _z (.z (`BoxComponent.BoxExtent` _box)))
  ;[1 1 1] Spawn lasers
  (for _index (range (+ _returnvalue 1))
    (bind _returnvalue_2 (`AddComponent|NODE_AddChildActorComponent-0` :`RelativeTransform` (`KismetMathLibrary.MakeTransform` (`KismetMathLibrary.MakeVector` 0.0 0.0 (`KismetMathLibrary.Lerp` (- 0.0 _z) _z (/ (`KismetMathLibrary.Conv_IntToDouble` _index) (`KismetMathLibrary.Conv_IntToDouble` _returnvalue)))) (struct) (`KismetMathLibrary.MakeVector` 1.0 1.0 (/ 1.0 (.z (`SceneComponent.K2_GetComponentScale` _box)))))))
    (`ChildActorComponent.SetChildActorClass` _returnvalue_2 "/Game/Environment/Laser_BP.Laser_BP_C")))