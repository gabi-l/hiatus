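; Goal pickup actor that a Runner reaches by overlapping its collider.
; Tick spins the collider and bobs it with a sine-driven world offset, which is added each frame without delta-time scaling.
; On authority only, the first Runner overlap sets a one-shot achieved flag, then OnGoalAchived hides the static mesh and calls GoalAchived.
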(event `self.ReceiveTick`
  (params (DeltaSeconds :type "Float (single-precision)"))
  ;[1 1 1] Plus Value
  (`SceneComponent.K2_AddWorldRotation` (`self.Collider`) (* (`self.RotationSpeed`) DeltaSeconds) false false)
  (`SceneComponent.K2_AddWorldOffset` (`self.Collider`) (`KismetMathLibrary.MakeVector` 0.0 0.0 (* (`self.Amplitude`) (`KismetMathLibrary.Sin` (* (`GameplayStatics.GetTimeSeconds`) (`self.WaveSpeed`))))) false false))

(event `self.Collider.OnComponentBeginOverlap`
  (params (OverlappedComponent :type "PrimitiveComponent Object Reference") (OtherActor :type "Actor Object Reference") (OtherComp :type "PrimitiveComponent Object Reference") (OtherBodyIndex :type Integer) (bFromSweep :type Boolean) (SweepResult :type "HitResult Structure (by ref)"))
  (`/Engine/EditorBlueprintResources/ActorMacros.Switch Has Authority`
    (:`Authority`
      (cast `/Game/Characters/Runner` OtherActor)
      (if (not (`self.IsAchived`))
        (set `self.IsAchived` true)
        (`self.OnGoalAchived`)))))

(event `OnGoalAchived`
  (`SceneComponent.SetVisibility` (`self.StaticMesh`) false false)
  (`self.GoalAchived`))

(fn `UserConstructionScript`)