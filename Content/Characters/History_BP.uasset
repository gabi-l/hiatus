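; History component for a Runner character, sketching a rewind system that records past mesh transforms and shows them as a ghost.
; Record samples the owner's mesh transform on a looping delay, and scrub direction and speed move a clamped index through that history.
; Ghost and timed-clone events spawn skeletal mesh actors using GetGhostTransform.
; BeginPlay and Tick are empty, internal event calls are disconnected, and GetGhostTransform's interpolation is unwired.
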(event `self.ReceiveBeginPlay`
  ;[1 0.02 0.02] Begin
)

(event `self.ReceiveTick`
  (params (DeltaSeconds :type "Float (single-precision)"))
  ;[1 0.01 0.01] Event Tick
)

(event `Record`
  ;[1 1 1] Record
  (bind _asrunner (cast `/Game/Characters/Runner` (`self.GetOwner`)))
  (`KismetArrayLibrary.Array_Add` (`self.Transforms`) (`SceneComponent.K2_GetComponentToWorld` (`/Game/Characters/Runner.SkeletalMesh` _asrunner)) :!label _label)
  (`KismetSystemLibrary.Delay` (/ 1.0 (`self.Frequency (f/s)`)))
  (goto _label))

(event `Clear`
  ;[1 1 1] Clear
  (`KismetArrayLibrary.Array_Clear` (`self.Transforms`)))

(event `Scrub`
  (params (Direction :type "Float (double-precision)"))
  ;[1 1 1] Scrub
  (set `self.Direction` Direction))

(event `StopScrubbing`
  ;[1 1 1] Stop Scrubbing
  (set `self.Direction` 0.0))

(event `AdjustIndex`
  ;[1 1 1] Adjust Index
  (set `self.Index` (`KismetMathLibrary.FClamp` (+ (* (`self.Direction`) (`self.Speed`) (`GameplayStatics.GetWorldDeltaSeconds`)) (`self.Index`)) 0.0 (`KismetMathLibrary.Conv_IntToDouble` (`KismetArrayLibrary.Array_Length` (`self.Transforms`))))))

(event `Spawn Ghost`
  ;[1 1 1] Spawn Ghost
  (bind _returnvalue (`|SpawnActorFromClass` "/Script/Engine.SkeletalMeshActor" (`Actor.GetTransform` (`self.GetOwner`)) "AlwaysSpawn" "OverrideRootScale"))
  (bind _output_get (set `self.Ghost` _returnvalue))
  (`SkinnedMeshComponent.SetSkinnedAssetAndUpdate` (`SkeletalMeshActor.SkeletalMeshComponent` _output_get) "/Game/Characters/SK_Coureur.SK_Coureur" true))

(event `Update Ghost`
  ;[1 1 1] Update Ghost
  (`SceneComponent.K2_SetWorldTransform` (`SkeletalMeshActor.SkeletalMeshComponent` (`self.Ghost`)) (`self.Get Ghost Transform`) false false))

(event `Create Clone`
  ;[1 1 1] Create Clone
  (bind _returnvalue (`|SpawnActorFromClass` "/Script/Engine.SkeletalMeshActor" (`self.Get Ghost Transform`) "AlwaysSpawn" "OverrideRootScale"))
  (`Actor.SetLifeSpan` _returnvalue (`self.Clone Lifetime`))
  (`SkinnedMeshComponent.SetSkinnedAssetAndUpdate` (`SkeletalMeshActor.SkeletalMeshComponent` _returnvalue) "/Game/Characters/SK_Coureur.SK_Coureur" true))