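; Ghost character that plays spawn and loop sounds and flashes while overlapping a Button_BP.
; Overlap begin and end toggle flashing and call target handlers; ending resets glow to minimum.
; While flashing, Tick writes FindGlowIntensity to a dynamic material created at construction; that function holds a sine-based lerp shown as unused.
; The Old graph retains Die, which destroys the actor, plus disconnected path-replay logic interpolating recorded transforms over a lifetime.
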(event `self.ReceiveBeginPlay`
  ;[1 1 1] Play Sound
  (`AudioComponent.Play` (`self.SpawnSound`) 0.0)
  (`AudioComponent.Play` (`self.LoopSound`) 0.0))

(event `self.ReceiveActorBeginOverlap`
  (params (OtherActor :type "Actor Object Reference"))
  ;[1 1 1] Activate flashing on overlap with button
  (cast `/Game/Environment/Button_BP` OtherActor)
  (set `self.IsFlashing` true)
  (`self.BeginOverlapTarget`)
  (set `self.FlashingStartTime` (`GameplayStatics.GetTimeSeconds`)))

(event `self.ReceiveActorEndOverlap`
  (params (OtherActor :type "Actor Object Reference"))
  ;[1 1 1] Deactivate flashing on overlap with button
  (cast `/Game/Environment/Button_BP` OtherActor)
  (set `self.IsFlashing` false)
  (`self.EndOverlapTarget`)
  (`MeshComponent.SetScalarParameterValueOnMaterials` (`self.SkeletalMesh`) (`self.GlowParameterName`) (`self.MinGlowIntesity`)))

(event `self.ReceiveTick`
  (params (DeltaSeconds :type "Float (single-precision)"))
  (if (`self.IsFlashing`)
    ;[1 1 1] Set glow intensity of material
    (`MaterialInstanceDynamic.SetScalarParameterValue` (`self.GhostDynMaterial`) (`self.GlowParameterName`) (`KismetMathLibrary.Lerp` (`self.MinGlowIntesity`) (`self.MaxGlowIntesity`) (/ (+ (`KismetMathLibrary.Sin` (* (- (`GameplayStatics.GetTimeSeconds`) (`self.FlashingStartTime`)) (`self.GlowSpeed`))) 1.0) 2.0)))))

(event `Die`
  (`self.K2_DestroyActor`))

(fn `UserConstructionScript`
  (bind _returnvalue (`PrimitiveComponent.CreateDynamicMaterialInstance` (`self.SkeletalMesh`) 0 "/Game/Assets/Materials/Ghost.Ghost"))
  (set `self.GhostDynMaterial` _returnvalue))