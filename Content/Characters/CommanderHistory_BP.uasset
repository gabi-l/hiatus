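; History component on the Commander that records the Runner's path and lets the player scrub back along it to place a timed clone.
; A delay loop samples Runner transforms at a fixed frequency, skipping unchanged poses and death rewinds, and spawns indicators shown while scrubbing.
; Scrub mode moves a short-lived ghost by interpolating samples within the rewind window; target overlaps flash the HUD pause button.
; Creating a clone or ghost expiry returns to normal mode.
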(event `LaunchHistory`
  ;[1 1 1] Begin
  (`|ExecutionSequence`
    (:`then_0`
      (`self.Record`))
    (:`then_1`
      (set `self.IsStarted` true))
    (:`then_2`
      (`self.Set Indicators Visibility` false))))

(event `self.ReceiveTick`
  (params (DeltaSeconds :type "Float (single-precision)"))
  ;[1 1 1] Event Tick
  (if (`self.IsStarted`)
    (switch `/Game/Characters/HistoryState` (`self.History State`)
      (:`NewEnumerator1`
        (`|ExecutionSequence`
          (:`then_0`
            (`self.AdjustIndex`))
          (:`then_1`
            (`self.Update Ghost`)))))))

(event `Record`
  (bind _transforms (`self.Transforms`))
  ;[1 1 1] Record
  (bind _ascommander_bp (cast `/Game/Characters/Commander_BP` (`self.GetOwner`)))
  (bind _runner (`/Game/Characters/Commander_BP.Runner` _ascommander_bp))
  (bind _returnvalue (`KismetMathLibrary.MakeTransform` (.location (`Actor.GetTransform` _runner)) (`SceneComponent.K2_GetComponentRotation` (`/Game/Characters/Runner.SkeletalMesh` _runner)) (.scale (`Actor.GetTransform` _runner))))
  (`KismetArrayLibrary.Array_Add` (`self.Transforms`) _returnvalue :!label _label)
  (`self.CreateHistoryIndicator` _returnvalue)
  (set `self.Last Record Time` (`GameplayStatics.GetTimeSeconds`))
  (`KismetSystemLibrary.Delay` (/ 1.0 (`self.Frequency (f/s)`)) :!label _label_2)
  (if (or (`self.IsDeathRewinding`) (`KismetMathLibrary.NearlyEqual_TransformTransform` _returnvalue (`KismetArrayLibrary.Array_Get` _transforms (`KismetArrayLibrary.Array_LastIndex` _transforms)) 0.0001 0.1))
    (goto _label_2)
    (else
      (goto _label))))

(event `Clear`
  ;[1 1 1] Fuck
  (`self.Clear Multicast`))

(event `Scrub`
  (params (Direction :type "Float (double-precision)"))
  ;[1 1 1] Scrub
  (switch `/Game/Characters/HistoryState` (`self.History State`)
    (:`NewEnumerator0`
      (if (< Direction 0.0)
        (set `self.Direction` Direction)
        (`self.StateChange_Scrub`)))
    (:`NewEnumerator1`
      (set `self.Direction` Direction))))

(event `StopScrubbing`
  ;[1 1 1] Stop Scrubbing
  (set `self.Direction` 0.0))

(event `Clear Multicast`
  ;[1 1 1] Clear
  (`KismetArrayLibrary.Array_Clear` (`self.Transforms`))
  (for _array_element (`self.HistoryIndicators`)
    (`Actor.K2_DestroyActor` _array_element))
  (`KismetArrayLibrary.Array_Clear` (`self.HistoryIndicators`)))

(event `AdjustIndex`
  (bind _returnvalue (`KismetMathLibrary.Conv_IntToDouble` (`KismetArrayLibrary.Array_Length` (`self.Transforms`))))
  (bind _returnvalue_2 (- _returnvalue (- (* (`self.Frequency (f/s)`) (`self.Max Rewind Time (s)`)) (`KismetMathLibrary.FClamp` (* (`self.Get Time Since Last Record`) (`self.Frequency (f/s)`))))))
  ;[1 1 1] Adjust Index
  (set `self.Index` (`KismetMathLibrary.FClamp` (+ (* (`self.Direction`) (`self.Scrub Speed`) (`GameplayStatics.GetWorldDeltaSeconds`)) (`self.Index`)) (`KismetMathLibrary.SelectFloat` _returnvalue_2 0.0 (> _returnvalue_2 0.0)) _returnvalue)))

(event `Spawn Ghost`
  (bind _transforms (`self.Transforms`))
  ;[1 1 1] Spawn Ghost
  (bind _returnvalue (`|SpawnActorFromClass` "/Game/Characters/Ghost_BP.Ghost_BP_C" (`KismetArrayLibrary.Array_Get` _transforms (`KismetArrayLibrary.Array_LastIndex` _transforms)) "AlwaysSpawn" "OverrideRootScale"))
  (bind _output_get (set `self.Ghost` _returnvalue))
  (`Actor.SetLifeSpan` _output_get (`self.Scrub Time (s)`))
  (add `Actor.OnDestroyed` _output_get (delegate `Scrub Time Over`))
  (add `/Game/Characters/Ghost_BP.BeginOverlapTarget` _output_get (delegate `GhostBeginOverlapTarget`))
  (add `/Game/Characters/Ghost_BP.EndOverlapTarget` _output_get (delegate `GhostEndOverlapTarget`)))

(event `Destroy Ghost`
  (bind _ghost (`self.Ghost`))
  ;[1 1 1] Destroy Ghost
  (if (`KismetSystemLibrary.IsValid` _ghost)
    (remove `Actor.OnDestroyed` _ghost (delegate `Scrub Time Over`))
    (`Actor.K2_DestroyActor` _ghost)))

(event `Update Ghost`
  ;[1 1 1] Update Ghost
  (bind _transform (`self.Get Ghost Transform`))
  (`Actor.K2_SetActorTransform` (`self.Ghost`) _transform false false))

(event `Scrub Time Over`
  (params (DestroyedActor :type "Actor Object Reference"))
  ;[1 1 1] Spawn Ghost
  (`self.StateChange_Normal`))

(event `GhostBeginOverlapTarget`
  ;[1 1 1] Ghost feedback indicator when overlapping target objects
  (bind _ascommander_bp (cast `/Game/Characters/Commander_BP` (`self.GetOwner`)))
  (bind _hud (`/Game/Characters/Commander_BP.HUD` _ascommander_bp))
  (if (`KismetSystemLibrary.IsValid` _hud)
    (`/Game/UI/Game/Controls_BP.StartFlashingPauseButton` (`/Game/UI/Game/CommanderHUD_BP.Controls` _hud))))

(event `GhostEndOverlapTarget`
  ;[1 1 1] Ghost feedback indicator when overlapping target objects
  (bind _ascommander_bp (cast `/Game/Characters/Commander_BP` (`self.GetOwner`)))
  (bind _hud (`/Game/Characters/Commander_BP.HUD` _ascommander_bp))
  (if (`KismetSystemLibrary.IsValid` _hud)
    (`/Game/UI/Game/Controls_BP.EndFlashingPauseButton` (`/Game/UI/Game/CommanderHUD_BP.Controls` _hud))))

(event `Create Clone Button Press`
  ;[1 1 1] Create Clone Button Press
  (`self.DestroyClone`)
  (`self.Spawn Clone`)
  (`self.StateChange_Normal`))

(event `Spawn Clone`
  (bind _transforms (`self.Transforms`))
  ;[1 1 1] Spawn Clone
  (bind _transform (`self.Get Ghost Transform`))
  (bind _returnvalue (`|SpawnActorFromClass` "/Game/Characters/Clone_BP.Clone_BP_C" (select `/Game/Characters/HistoryState` (`self.History State`) :`NewEnumerator0` (`KismetArrayLibrary.Array_Get` _transforms (`KismetArrayLibrary.Array_LastIndex` _transforms)) :`NewEnumerator1` _transform) "AlwaysSpawn" "OverrideRootScale"))
  (bind _output_get (set `self.Clone` _returnvalue))
  (`Actor.SetLifeSpan` _output_get (`self.Clone Lifetime (s)`))
  (bind _ascommander_bp (cast `/Game/Characters/Commander_BP` (`self.GetOwner`)))
  (`AudioComponent.Play` (`/Game/Characters/Commander_BP.CloneClockSound` _ascommander_bp) 0.0))

(event `DestroyClone`
  (bind _clone (`self.Clone`))
  ;[1 1 1] Destroy Clone
  (if (`KismetSystemLibrary.IsValid` _clone)
    (`Actor.K2_DestroyActor` _clone)))

(event `CreateHistoryIndicator`
  (params (Transform :type "Transform Structure"))
  ;[1 1 1] Create History Indicators
  (bind _returnvalue (`|SpawnActorFromClass` "/Game/Environment/HistoryIndicator_BP.HistoryIndicator_BP_C" Transform "Undefined" "OverrideRootScale"))
  (`KismetArrayLibrary.Array_Add` (`self.HistoryIndicators`) _returnvalue)
  (`self.SetIndicatorVisibility` _returnvalue (select `/Game/Characters/HistoryState` (`self.History State`) :`NewEnumerator1` true)))

(event `RunnerDies`
  ;[1 1 1] Runner Dies
  (`self.Clear`))

(event `SetIndicatorVisibility`
  (params (HistoryIndicator :type "/Game/Environment/HistoryIndicator_BP Object Reference") (Visibility :type Boolean))
  ;[1 1 1] Set one indicator visibility
  (`SceneComponent.SetVisibility` (`/Game/Environment/HistoryIndicator_BP.DefaultSceneRoot` HistoryIndicator) Visibility true))

(event `Set Indicators Visibility`
  (params (Visible :type Boolean))
  ;[1 1 1] Set Indicators Visibility
  (for _array_element (`self.HistoryIndicators`)
    (`SceneComponent.SetVisibility` (`/Game/Environment/HistoryIndicator_BP.DefaultSceneRoot` _array_element) Visible true)))

(event `StateChange_Normal`
  ;[1 1 1] State Change : Normal
  (set `self.History State` "NewEnumerator0")
  (`self.Destroy Ghost`)
  (`self.Set Indicators Visibility` false))

(event `StateChange_Scrub`
  ;[1 1 1] State Change : Scrub
  (set `self.History State` "NewEnumerator1")
  (`self.Spawn Ghost`)
  (set `self.Index` (`KismetMathLibrary.Conv_IntToDouble` (`KismetArrayLibrary.Array_LastIndex` (`self.Transforms`))))
  (`self.Set Indicators Visibility` true))

(fn `Get Clone Timer`
  (returns (`Time Left (s)` :type "Float (double-precision)"))
  (bind _clone (`self.Clone`))
  (return (`KismetMathLibrary.SelectFloat` (`Actor.GetLifeSpan` _clone) 0.0 (`KismetSystemLibrary.IsValid` _clone))))

(fn `Get Ghost Timer`
  (returns (`Time Left (s)` :type "Float (double-precision)"))
  (bind _ghost (`self.Ghost`))
  (return (`KismetMathLibrary.SelectFloat` (`Actor.GetLifeSpan` _ghost) 0.0 (`KismetSystemLibrary.IsValid` _ghost))))

(fn `Get Ghost Transform`
  (returns (Transform :type "Transform Structure"))
  (bind _index (`self.Index`))
  (bind _transforms (`self.Transforms`))
  (bind _returnvalue (`KismetMathLibrary.FTrunc` _index))
  (bind _returnvalue_2 (- (`KismetArrayLibrary.Array_Length` _transforms) 1))
  ;[1 1 1] Get Ghost Transform
  (bind _ascommander_bp (cast `/Game/Characters/Commander_BP` (`self.GetOwner`)))
  (return (`KismetMathLibrary.SelectTransform` (`KismetMathLibrary.TLerp` (`KismetArrayLibrary.Array_Get` _transforms (`KismetMathLibrary.Clamp` _returnvalue 0 _returnvalue_2)) (`KismetArrayLibrary.Array_Get` _transforms (`KismetMathLibrary.Clamp` (+ _returnvalue 1) 0 _returnvalue_2)) (`KismetMathLibrary.FClamp` (- _index (`KismetMathLibrary.Conv_IntToDouble` _returnvalue)))) (`Actor.GetTransform` (`/Game/Characters/Commander_BP.Runner` _ascommander_bp)) (> (`KismetArrayLibrary.Array_Length` (`self.Transforms`)) 0))))