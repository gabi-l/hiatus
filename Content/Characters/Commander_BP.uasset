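; Commander player pawn that oversees the Runner with a pannable camera, selects objects and controls time scrubbing and clone creation.
; Input moves it at zoom-scaled speed or lerps focus onto the Runner, while floor traces smooth its height.
; Each tick, camera traces drive selection tooltips and fade occluding walls.
; It also creates the HUD, counts achieved goals to travel levels, gates tutorial controls and launches history on authority.
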(event `self.ReceiveBeginPlay`
  ;[1 1 1] Initialization
  (`|ExecutionSequence`
    (:`then_0`
      (if (or (`self.IsLocallyControlled`) (`self.IsShowingHUD`))
        (`self.InitializeHUD`)
        (bind _outactors (`GameplayStatics.GetAllActorsOfClass` "/Game/Environment/Goal_BP.Goal_BP_C"))
        (bind _output_get (set `self.GoalsCount` (`KismetArrayLibrary.Array_Length` _outactors)))
        (`/Game/UI/Game/CommanderHUD_BP.SetGoalsCount` (`self.HUD`) _output_get)
        (for _array_element _outactors
          (add `/Game/Environment/Goal_BP.GoalAchived` _array_element (delegate `GoalAchived`)))
        (bind _outactors_2 (`GameplayStatics.GetAllActorsOfClass` "/Game/Environment/TooltipTrigger_BP.TooltipTrigger_BP_C"))
        (for _array_element_2 _outactors_2
          (add `/Game/Environment/TooltipTrigger_BP.ShowIndicator` _array_element_2 (delegate `ShowIndicator`)))
        (`self.GetCurrentLevelIndex`)))
    (:`then_1`
      ;;[1 1 1] Try to set runner reference
      (`self.GetAndSetCharacterReferences`))))

(event `GetCurrentLevelIndex`
  ;[1 1 1] Get current level index
  (bind _asgame_info_instance (cast `/Game/GameInstance/GameInfoInstance` (`GameplayStatics.GetGameInstance`)))
  (`self.RefreshCurrentLevelIndex` (`/Game/GameInstance/GameInfoInstance.CurrentLevelIndex` _asgame_info_instance) (`KismetArrayLibrary.Array_Length` (`/Game/GameInstance/GameInfoInstance.Levels` _asgame_info_instance))))

(event `ShowIndicator`
  (params (Control :type "/Game/UI/Game/ControlsType Enum"))
  ;[1 1 1] Shows indicator
  (`/Game/UI/Game/Controls_BP.ShowIndicator` (`/Game/UI/Game/CommanderHUD_BP.Controls` (`self.HUD`)) Control)
  (switch `/Game/UI/Game/ControlsType` Control
    (:`NewEnumerator0`
      (set `self.PauseEnabled` true))
    (:`NewEnumerator1`
      (set `self.TimeControlsEnabled` true))))

(event `GoalAchived`
  ;[1 1 1] Goals reached
  (bind _result (`/Engine/EditorBlueprintResources/StandardMacros.IncrementInt` (`self.GoalsAchived`))
    (:`  `
      (`/Game/UI/Game/CommanderHUD_BP.SetGoalsAchived` (`self.HUD`) _result)
      (if (== (`self.GoalsAchived`) (`self.GoalsCount`))
        (`self.LoadNextLevel`)))))

(event `RefreshCurrentLevelIndex`
  (params (Index :type Integer) (LevelsCount :type Integer))
  ;[1 1 1] Get current level index
  (if (!= Index 0)
    (`/Game/UI/Game/Controls_BP.ShowHUD` (`/Game/UI/Game/CommanderHUD_BP.Controls` (`self.HUD`)))
    (if (== Index (- LevelsCount 1))
      (bind _returnvalue (`|CreateWidget` "/Game/UI/widgets/Credits.Credits_C"))
      (`UserWidget.AddToViewport` _returnvalue 100)
      (`Widget.SetVisibility` _returnvalue "Visible")
      (`/Game/UI/widgets/Credits.PlayCredits` _returnvalue))
    (else
      (set `self.IsTutorialMode` true))))

(event `AllGoalsReached`
  ;[1 1 1] Goals reached
  ;;[1 0.27 0.27] Old code
  (bind _outactors (`GameplayStatics.GetAllActorsWithTag` "END"))
  (if (> (`KismetArrayLibrary.Array_Length` _outactors) 0)
    (bind _asdoor_bp (cast `/Game/Environment/Door_BP` (`KismetArrayLibrary.Array_Get` _outactors)))
    (`/Game/Environment/Door_BP.Open` _asdoor_bp)))

(event `InitializeHUD`
  ;[1 1 1] Initializes HUD
  (bind _returnvalue (`|CreateWidget` "/Game/UI/Game/CommanderHUD_BP.CommanderHUD_BP_C"))
  (set `self.HUD` _returnvalue)
  (`UserWidget.AddToViewport` (`self.HUD`) 0)
  (`Widget.SetVisibility` (`self.HUD`) "Visible"))

(event `self.ReceiveTick`
  (params (DeltaSeconds :type "Float (single-precision)"))
  (bind _desiredposition (`self.DesiredPosition`))
  (bind _lerpduration (`self.LerpDuration`))
  (bind _camera (`self.Camera`))
  (bind _returnvalue (`SceneComponent.K2_GetComponentLocation` _camera))
  (bind _returnvalue_2 (/ (- (`GameplayStatics.GetTimeSeconds`) (`self.StartTime`)) _lerpduration))
  (bind _returnvalue_3 (`KismetMathLibrary.VLerp` (`self.StartPosition`) (`self.DesiredPosition`) _returnvalue_2))
  ;[1 1 1] Try to initialize history (will not duplicate the initialization)
  (`self.InitializeHistory`)
  (`|ExecutionSequence`
    (:`then_0`
      ;[1 1 1] Detects a selectable object
      (if (!= (`self.HUD`) null)
        (bind (_outhit _returnvalue_4) (`KismetSystemLibrary.SphereTraceSingle_NEW` _returnvalue (+ _returnvalue (* (`KismetMathLibrary.GetForwardVector` (`SceneComponent.K2_GetComponentRotation` _camera)) (`self.RaycastDistance`))) 200.0 "TraceTypeQuery3"))
        (bind (_bblockinghit _binitialoverlap _time _location _impactpoint _normal _impactnormal _physmat _hitactor) (`GameplayStatics.BreakHitResult` _outhit))
        ;[1 1 1] Executes the release action
        (if (and (!= (`self.CurrentSelection`) null) (== _hitactor null))
          (`self.ReleaseAction` (`self.CurrentSelection`))
          (set `self.IsActivating` false))
        ;[1 1 1] Displays a tooltip associated with the selectable object
        (set `self.CurrentSelection` _hitactor)
        (if _returnvalue_4
          (if (`self.NewSelectionOccurred`)
            (set `self.NewSelectionOccurred` false)
            (bind _infos (message `/Game/Shared/SelectableObject_BP.GetInformation` (`self.CurrentSelection`) false))
            (`/Game/UI/Game/CommanderHUD_BP.ShowTooltip` (`self.HUD`) _infos))
          (else
            (`/Game/UI/Game/CommanderHUD_BP.HideToolTip` (`self.HUD`))
            (set `self.NewSelectionOccurred` true)))))
    (:`then_1`
      (`self.Wall Visibility`))
    (:`then_2`
      (if (`self.IsLockingOnPosition`)
        (if (== _lerpduration 0.0)
          (`self.K2_SetActorLocation` _desiredposition :!label _label)
          (`SceneComponent.K2_SetWorldLocation` (`self.Camera`) _desiredposition false false)
          (set `self.IsLockingOnPosition` false)
          (elif (> _returnvalue_2 1.0)
            (goto _label)
            (else
              (`self.K2_SetActorLocation` _returnvalue_3)
              (`SceneComponent.K2_SetWorldLocation` (`self.Camera`) _returnvalue_3 false false))))))
    (:`then_3`
      (`self.Smooth Height` DeltaSeconds))))

(event `FocusOnRunnerEvent`
  (params (NewParam :type "Vector Structure") (NewParam2 :type "Float (double-precision)"))
  ;[1 1 1] Focus on runner pressed
  (`self.FocusCommanderOn` NewParam NewParam2))

(event `InputAxis|ForwardBackward`
  (params (AxisValue :type "Float (single-precision)"))
  (bind _camera (`self.Camera`))
  ;[1 1 1] Controls
  (bind _mouvmentcorrection (`self.AjustMaxSpeed` (`CameraComponent.OrthoWidth` _camera) AxisValue))
  (`self.K2_SetActorLocation` (+ (* (* (`KismetMathLibrary.GetForwardVector` (`KismetMathLibrary.MakeRotator` 0.0 0.0 (.yaw (`SceneComponent.K2_GetComponentRotation` _camera)))) _mouvmentcorrection) (* (`self.Speed`) (`GameplayStatics.GetWorldDeltaSeconds`))) (`self.K2_GetActorLocation`))))

(event `InputAction|FocusRunner`
  (params (Key :type "Key Structure" :default "AnyKey"))
  ;[1 1 1] Focus on runner pressed
  (:`Pressed`
    (`self.FocusCommanderOn` (`self.K2_GetActorLocation` (`self.Runner`)) (`self.DeltaTimeOnFocus`))
    (`/Game/UI/Game/LocationButton_BP.PressButton` (`/Game/UI/Game/CommanderHUD_BP.LocationButton` (`self.HUD`)))))

(event `InputAction|SelectObject`
  (params (Key :type "Key Structure" :default "AnyKey"))
  ;[1 1 1] Executes the selection action on the selected object
  (:`Pressed`
    (if false
      _
      (elif (!= (`self.CurrentSelection`) null)
        (`/Game/UI/Game/CommanderHUD_BP.HideToolTip` (`self.HUD`))
        (bind _asselectable_actor (cast `/Game/Shared/SelectableActor` (`self.CurrentSelection`))
          (:`then`
            (add `/Game/Shared/SelectableActor.SelectionActionCompleted` _asselectable_actor (delegate `SelectionActionCompleted`))
            (message `/Game/Shared/SelectableObject_BP.PressAction` (`self.CurrentSelection`) false))
          (:`CastFailed`
            (message `/Game/Shared/SelectableObject_BP.PressAction` (`self.CurrentSelection`) false)
            (`self.SelectionActionCompleted`)))
        (set `self.IsActivating` true))))
  (:`Released`
    (if (!= (`self.CurrentSelection`) null)
      (`self.ReleaseAction` (`self.CurrentSelection`))
      (set `self.NewSelectionOccurred` true)
      (set `self.IsActivating` false))))

(event `InputAxis|StrafeRightLeft`
  (params (AxisValue :type "Float (single-precision)"))
  ;[1 1 1] Controls
  (bind _mouvmentcorrection (`self.AjustMaxSpeed` (`CameraComponent.OrthoWidth` (`self.Camera`)) AxisValue))
  (`self.K2_SetActorLocation` (+ (* (* (`KismetMathLibrary.GetRightVector` (`KismetMathLibrary.MakeRotator` 0.0 0.0 (.yaw (`SceneComponent.K2_GetComponentRotation` (`self.Camera`))))) _mouvmentcorrection) (* (`self.Speed`) (`GameplayStatics.GetWorldDeltaSeconds`))) (`self.K2_GetActorLocation`))))

(event `SelectionActionCompleted`
  (bind _currentselection (`self.CurrentSelection`))
  ;[1 1 1] Replication logic
  (bind _asselectable_actor (cast `/Game/Shared/SelectableActor` _currentselection)
    (:`then`
      (remove `/Game/Shared/SelectableActor.SelectionActionCompleted` _asselectable_actor (delegate `SelectionActionCompleted`)))
    (:`CastFailed`
      _))
  (`self.ConfirmAction` _currentselection))

(event `InputAction|SpawnIndicator`
  (params (Key :type "Key Structure" :default "AnyKey"))
  ;[1 1 1] Spaws the indicator
)

(event `ConfirmAction`
  (params (Actor :type "Actor Object Reference"))
  ;[1 1 1] Replication logic
  (message `/Game/Shared/SelectableObject_BP.CompleteAction` Actor false))

(event `ReleaseAction`
  (params (Actor :type "Actor Object Reference"))
  ;[1 1 1] Replication logic
  (message `/Game/Shared/SelectableObject_BP.ReleaseAction` Actor false))

(event `Get Runner Reference`
  ;[1 0 0] Gets the runner reference
  (add `/Game/Characters/Runner.GhostCreated` (`self.Runner`) (delegate `GhostCreated`)))

(event `LoadLevel`
  (params (LevelIndex :type Integer))
  ;[0.9852 1 0] Load Next Level
  (`self.ShowLoadingScreenOnEveryone`)
  (bind _asgameplay_pc (cast `/Game/GameInstance/GameplayPC` (`GameplayStatics.GetPlayerController` 0)))
  (`/Game/GameInstance/GameplayPC.TravelToLevel` _asgameplay_pc LevelIndex))

(event `GhostCreated`
  (params (Duration :type "Float (double-precision)"))
  ;[1 0 0] Shows the ghost indicator
  (`/Game/UI/Game/CommanderHUD_BP.ShowGhostIndicator` (`self.HUD`) Duration))

(event `LoadNextLevel`
  ;[0.9852 1 0] Load Next Level
  (`self.ShowLoadingScreenOnEveryone`)
  (bind _asgameplay_pc (cast `/Game/GameInstance/GameplayPC` (`GameplayStatics.GetPlayerController` 0)))
  (`/Game/GameInstance/GameplayPC.TravelToNextLevel` _asgameplay_pc))

(event `InputAxis|TimeScrubbing`
  (params (AxisValue :type "Float (single-precision)"))
  (bind _controls (`/Game/UI/Game/CommanderHUD_BP.Controls` (`self.HUD`)))
  ;[1 1 1] Time Controls
  (if (or (not (`self.IsTutorialMode`)) (`self.TimeControlsEnabled`))
    (`/Game/Characters/CommanderHistory_BP.Scrub` (`self.CommanderHistory_BP`) AxisValue)
    (if (`KismetSystemLibrary.IsValid` (`self.HUD`))
      (if (!= AxisValue 0.0)
        (if (> AxisValue 0.0)
          (`/Game/UI/Game/Controls_BP.ChangeRewingStatus` _controls false)
          (`/Game/UI/Game/Controls_BP.ChangeForwardStatus` _controls true)
          (else
            (`/Game/UI/Game/Controls_BP.ChangeForwardStatus` _controls false)
            (`/Game/UI/Game/Controls_BP.ChangeRewingStatus` _controls true)))
        (else
          (`/Game/UI/Game/Controls_BP.ChangeForwardStatus` _controls false)
          (`/Game/UI/Game/Controls_BP.ChangeRewingStatus` _controls false))))))

(event `ShowLoadingScreenOnEveryone`
  ;[0.9852 1 0] Load Next Level
  (`self.ShowLoadingScreenMulticast`))

(event `InputAction|Create_Clone`
  (params (Key :type "Key Structure" :default "AnyKey"))
  ;[1 1 1] Create Clone
  (:`Pressed`
    (if (or (not (`self.IsTutorialMode`)) (`self.PauseEnabled`))
      (`/Game/Characters/CommanderHistory_BP.Create Clone Button Press` (`self.CommanderHistory_BP`))
      (`/Game/UI/Game/Controls_BP.StartCountDown` (`/Game/UI/Game/CommanderHUD_BP.Controls` (`self.HUD`)) (`/Game/Characters/CommanderHistory_BP.Clone Lifetime (s)` (`self.CommanderHistory_BP`))))))

(event `ShowLoadingScreenMulticast`
  ;[0.9852 1 0] Load Next Level
  (bind _asgame_info_instance (cast `/Game/GameInstance/GameInfoInstance` (`GameplayStatics.GetGameInstance`)))
  (`/Game/GameInstance/GameInfoInstance.ShowLoadingScreen` _asgame_info_instance))

(event `Wall Visibility`
  (bind _camera (`self.Camera`))
  (bind _returnvalue (`SceneComponent.K2_GetComponentLocation` _camera))
  (bind _capsulecomponent (`Character.CapsuleComponent` (`self.Runner`)))
  ;[1 1 1] Hidden Walls
  (if (`self.IsLocallyControlled`)
    (`|ExecutionSequence`
      (:`then_0`
        (if (`KismetSystemLibrary.IsValid` (`self.Runner`))
          (bind _outhits (`KismetSystemLibrary.CapsuleTraceMulti_NEW` (`SceneComponent.K2_GetComponentLocation` (`self.Camera`)) (`SceneComponent.K2_GetComponentLocation` _capsulecomponent) (`CapsuleComponent.CapsuleRadius` _capsulecomponent) (`CapsuleComponent.CapsuleHalfHeight` _capsulecomponent) "TraceTypeQuery4"))
          (for _array_element _outhits
            (bind _asinvisible_wall_bp (cast `/Game/Environment/InvisibleWall_BP` (`.HitActor` (`GameplayStatics.BreakHitResult` _array_element))))
            (`/Game/Environment/InvisibleWall_BP.Set Translucent Object Visibility` _asinvisible_wall_bp true true))))
      (:`then_1`
        (bind _outhits_2 (`KismetSystemLibrary.SphereTraceMulti_NEW` _returnvalue (+ _returnvalue (* (`KismetMathLibrary.GetForwardVector` (`SceneComponent.K2_GetComponentRotation` _camera)) 30000.0)) 1000.0 "TraceTypeQuery4"))
        (for _array_element_2 _outhits_2
          (bind _asinvisible_wall_bp_2 (cast `/Game/Environment/InvisibleWall_BP` (`.HitActor` (`GameplayStatics.BreakHitResult` _array_element_2))))
          (`/Game/Environment/InvisibleWall_BP.Set Translucent Object Visibility` _asinvisible_wall_bp_2 true true))))))

(event `RunnerDies`
  ;[1 1 1] Called when the runner dies to ensure the commander is ready to continue
)

(event `InputAction|All_RespawnRunnerAfterDeath`
  (params (Key :type "Key Structure" :default "AnyKey"))
  ;[1 1 1] Commander ready check
)

(event `SetRunnerReadyToRespawnRunner`
  ;[1 1 1] Commander ready check
  (set `self.IsReadyToRespawnRunner` true))

(event `FocusOnRunner`
  (params (TargetPosition :type "Vector Structure") (DeltaTime :type "Float (double-precision)"))
  ;[1 1 1] No Comment
  (`self.FocusCommanderOn` TargetPosition DeltaTime))

(event `Smooth Height`
  (params (DeltatTime :type "Float (double-precision)"))
  (bind _returnvalue (`self.K2_GetActorLocation`))
  (bind _camera (`self.Camera`))
  ;[0 0.3328 1] Smooth Height
  (if (not (`self.IsLockingOnPosition`))
    (`|ExecutionSequence`
      (:`then_0`
        ;;[1 1 1] Check height at ray intersection
        (bind (_outhit _returnvalue_2) (`KismetSystemLibrary.LineTraceSingle` _returnvalue (+ _returnvalue (* (`SceneComponent.GetForwardVector` (`self.Camera`)) 10000)) "TraceTypeQuery5"))
        (if _returnvalue_2
          (bind _returnvalue_3 (+ (.z (`self.K2_GetActorLocation` (`.HitActor` (`GameplayStatics.BreakHitResult` _outhit)))) (`self.SmoothCommanderHeight`)))
          (bind _returnvalue_4 (`KismetMathLibrary.MakeVector` (.x (`self.K2_GetActorLocation`)) (.y (`self.K2_GetActorLocation`)) _returnvalue_3))
          ;;[1 1 1] Check height when the commander is going to be at the desired height
          (bind (_outhit_2 _returnvalue_5) (`KismetSystemLibrary.LineTraceSingle` _returnvalue_4 (+ _returnvalue_4 (* (`SceneComponent.GetForwardVector` (`self.Camera`)) 10000)) "TraceTypeQuery5"))
          ;;[1 1 1] Make sure the two heights don't fight by always taking the maximum
          (if _returnvalue_5
            (set `self.DesiredHeight` (`KismetMathLibrary.FMax` (+ (.z (`self.K2_GetActorLocation` (`.HitActor` (`GameplayStatics.BreakHitResult` _outhit_2)))) (`self.SmoothCommanderHeight`)) _returnvalue_3))
            (else
              (set `self.DesiredHeight` _returnvalue_3)))))
      (:`then_1`
        (if (not (`KismetMathLibrary.NearlyEqual_FloatFloat` (`self.DesiredHeight`) (`self.SmoothAverage`) 0.01))
          ;;[1 1 1] Interpolate to desired height
          (set `self.SmoothAverage` (`KismetMathLibrary.FInterpTo` (.z (`self.K2_GetActorLocation`)) (`self.DesiredHeight`) DeltatTime (`self.HeightSmoothSpeed`)))
          (`self.K2_SetActorLocation` (`KismetMathLibrary.MakeVector` (.x (`self.K2_GetActorLocation`)) (.y (`self.K2_GetActorLocation`)) (`self.SmoothAverage`)))
          (`SceneComponent.K2_SetWorldLocation` _camera (`KismetMathLibrary.MakeVector` (.x (`SceneComponent.K2_GetComponentLocation` _camera)) (.y (`SceneComponent.K2_GetComponentLocation` _camera)) (`self.SmoothAverage`)) false false))))))

(fn `AjustMaxSpeed`
  (params (CameraOrthoWidth :type "Float (double-precision)") (AxisValue :type "Float (double-precision)"))
  (returns (MouvmentCorrection :type "Float (double-precision)"))
  (return (* (/ CameraOrthoWidth 3900.0) AxisValue)))

(fn `FocusCommanderOn`
  (params (TargetPosition :type "Vector Structure") (DeltaTime :type "Float (double-precision)"))
  ;[1 1 1] Set variable used for interpolation
  (set `self.DesiredPosition` (+ TargetPosition (* (`SceneComponent.GetForwardVector` (`self.Camera`)) (* (`self.DistanceFromRunner`) -1))))
  (set `self.StartPosition` (`self.K2_GetActorLocation`))
  (set `self.StartTime` (`GameplayStatics.GetTimeSeconds`))
  (set `self.LerpDuration` DeltaTime)
  (set `self.IsLockingOnPosition` true))

(fn `GetAndSetCharacterReferences`
  ;[1 1 1] If not already initialize, initialize a reference on the runner if he exists. If so, trigger the initialization of the reference in the runner
  (if (not (`KismetSystemLibrary.IsValid` (`self.Runner`)))
    (bind _outactors (`GameplayStatics.GetAllActorsOfClass` "/Game/Characters/Runner.Runner_C"))
    (if (>= (`KismetArrayLibrary.Array_Length` _outactors) 0)
      (bind _item (`KismetArrayLibrary.Array_Get` _outactors))
      (if (`KismetSystemLibrary.IsValid` _item)
        (bind _output_get (set `self.Runner` _item))
        (`/Game/Characters/Runner.GetAndSetCharacterReferences` _output_get)
        (`self.Get Runner Reference`)
        (bind _asgame_info_instance (cast `/Game/GameInstance/GameInfoInstance` (`GameplayStatics.GetGameInstance`)))
        (`/Game/GameInstance/GameInfoInstance.HideLoadingScreen` _asgame_info_instance)))))

(fn `InitializeHistory`
  ;[1 1 1] Will initialize the history once the runner refercence is valid. The history will only be initialized once.
  (if (`self.IsHistoryInitialized`)
    (if (`KismetSystemLibrary.IsValid` (`self.Runner`))
      (`/Engine/EditorBlueprintResources/ActorMacros.Switch Has Authority`
        (:`Authority`
          (`/Game/Characters/CommanderHistory_BP.LaunchHistory` (`self.CommanderHistory_BP`))
          (`self.FocusCommanderOn` (`self.K2_GetActorLocation` (`self.Runner`)))
          (set `self.IsHistoryInitialized` false))))))

(fn `IsRunnerDead`
  (returns (IsRunnerDead :type Boolean))
  (bind _runner (`self.Runner`))
  (`/Engine/EditorBlueprintResources/StandardMacros.IsValid` _runner
    (:`Is Valid`
      (return (`/Game/Characters/Runner.IsDead` _runner)))
    (:`Is Not Valid`
      (return false))))

(fn `UserConstructionScript`)