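; DeadRunner_BP is a dead runner effect that animates the runner mesh's opacity as soon as it begins play.
; The construction script creates dynamic instances of the dead body and number materials on the Runner's two material slots.
; It also passes itself to the particle system as the VertSurfaceActor parameter, pointing particles at its own mesh surface.
; On BeginPlay, the Death timeline drives the Opacity parameter on both materials.
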(event `self.ReceiveBeginPlay`
  (bind (_direction _opacity) (`Timeline|Death` :!via `PlayFromStart`)
    (:`Update`
      (`MaterialInstanceDynamic.SetScalarParameterValue` (`self.DynMat1`) "Opacity" _opacity)
      (`MaterialInstanceDynamic.SetScalarParameterValue` (`self.DynMat2`) "Opacity" _opacity))))

(fn `UserConstructionScript`
  (`ParticleSystemComponent.SetActorParameter` (`self.ParticleSystem`) "VertSurfaceActor" self)
  (bind _returnvalue (`PrimitiveComponent.CreateDynamicMaterialInstance` (`self.Runner`) 0 "/Game/Assets/Materials/DeadRunner_Mat.DeadRunner_Mat"))
  (set `self.DynMat1` _returnvalue)
  (bind _returnvalue_2 (`PrimitiveComponent.CreateDynamicMaterialInstance` (`self.Runner`) 1 "/Game/Characters/Materials/NUmber_Dead.NUmber_Dead"))
  (set `self.DynMat2` _returnvalue_2))