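; Clone character that plays a spawn sound and carries a glowing material whose flashing speed depends on its remaining life span.
; Construction creates the dynamic material and records birth time.
; On authority, Tick picks normal or fast glow speed by a remaining-time threshold; Tick also writes FindGlowIntensity's result to the material.
; FindGlowIntensity holds a sine-based min-max lerp over age and glow speed, shown as unconnected.
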(event `self.ReceiveBeginPlay`
  (`AudioComponent.Play` (`self.SpawnSound`) 0.0))

(event `self.ReceiveTick`
  (params (DeltaSeconds :type "Float (single-precision)"))
  (`|ExecutionSequence`
    (:`then_0`
      (`/Engine/EditorBlueprintResources/ActorMacros.Switch Has Authority`
        (:`Authority`
          (set `self.GlowSpeed` (`KismetMathLibrary.SelectFloat` (`self.GlowSpeedNormal`) (`self.GlowSpeedFast`) (> (`self.GetLifeSpan`) (`self.TimeRemainingWhenFlashingStarts`)))))))
    (:`then_1`
      ;[1 1 1] Set glow intensity of material
      (`MaterialInstanceDynamic.SetScalarParameterValue` (`self.CloneDynMaterial`) (`self.GlowParameterName`) (`KismetMathLibrary.Lerp` (`self.MinGlowIntensiity`) (`self.MaxGlowIntensity`) (/ (+ (`KismetMathLibrary.Sin` (* (- (`GameplayStatics.GetTimeSeconds`) (`self.BirthTime`)) (`self.GlowSpeed`))) 1.0) 2.0))))))

(fn `UserConstructionScript`
  (bind _returnvalue (`PrimitiveComponent.CreateDynamicMaterialInstance` (`self.SkeletalMesh`) 0 "/Game/Assets/Materials/Clone.Clone"))
  (set `self.CloneDynMaterial` _returnvalue)
  (set `self.BirthTime` (`GameplayStatics.GetTimeSeconds`)))