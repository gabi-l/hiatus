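; Projectile actor for the turret AI that kills runners on contact.
; ShootAt launches it by setting the SphereBV physics velocity toward a target location at a given speed.
; Overlaps are resolved only on the server and ignore turret characters.
; An actor with the killable tag that casts to Runner dies and the bullet is destroyed; untagged or invalid hits just destroy the bullet.
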(event `DestroyBullet`
  ;[1 1 1] Destroy the bullet
  (`self.K2_DestroyActor`))

(event `self.SphereBV.OnComponentBeginOverlap`
  (params (OverlappedComponent :type "PrimitiveComponent Object Reference") (OtherActor :type "Actor Object Reference") (OtherComp :type "PrimitiveComponent Object Reference") (OtherBodyIndex :type Integer) (bFromSweep :type Boolean) (SweepResult :type "HitResult Structure (by ref)"))
  ;[1 1 1] Check collision for runner or ghost and if not just delete the projectile
  (`/Engine/EditorBlueprintResources/ActorMacros.Switch Has Authority`
    (:`Authority`
      (cast `/Game/Characters/Enemies/TurretAI/TurretAI_Character` OtherActor
        (:`CastFailed`
          (if (`KismetSystemLibrary.IsValid` OtherActor)
            (if (`self.ActorHasTag` OtherActor (`self.KillableActorTag`))
              (bind _asrunner (cast `/Game/Characters/Runner` OtherActor))
              (`/Game/Characters/Runner.Die` _asrunner)))
          (`self.DestroyBullet`))))))

(event `ShootAt`
  (params (TargetLocation :type "Vector Structure") (LaunchSpeed :type "Float (double-precision)"))
  ;[1 1 1] Launch the projectile
  (`PrimitiveComponent.SetPhysicsLinearVelocity` (`self.SphereBV`) (* (`KismetMathLibrary.Normal` (- TargetLocation (`self.K2_GetActorLocation`))) LaunchSpeed) false "None"))

(fn `UserConstructionScript`)